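; BP_Player is the player pawn in the drone game, handling movement, look and firing input.
; On BeginPlay it adds the Enhanced Input mapping context, hands its muzzle to the weapon component and binds health's death event to destroy the actor.
; Move input is rotated by actor yaw only before reaching the movement component, rotate input drives controller yaw and pitch, and fire input starts and stops the weapon.
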(event Custom|Death
  (Actor|DestroyActor))

(event EventBeginPlay
  (bind _asplayer_controller (Utilities|Casting|CastToPlayerController (Pawn|GetController)))
  (Input|AddMappingContext (PlayerController|LocalPlayerSubsystems|GetEnhancedInputLocalPlayerSubsystem _asplayer_controller) "/Game/DroneGame/Blueprints/Player/Input/IMC_Player.IMC_Player" 0 "(bIgnoreAllPressedKeysUntilRelease=True,bForceImmediately=False,bNotifyUserSettings=False)")
  (Variables|/Script/DroneGame.WeaponComponent|SetMuzzleComponent (Variables|Default|GetWeaponComponent) (Variables|Default|GetMuzzle))
  (EventDispatchers|BindEventtoOnDeath (Variables|Default|GetHealthComponent) (delegate Custom|Death)))

(event Input|EnhancedActionEvents|EnhancedInputActionIA_Move
  (params (ActionValue :type Vector :default "0, 0, 0") (ElapsedSeconds :type Float%20%28double-precision%29) (TriggeredSeconds :type Float%20%28double-precision%29) (InputAction :type Input%20Action%20Object%20Reference :default "/Game/DroneGame/Blueprints/Player/Input/IA_Move.IA_Move"))
  (Class|PawnMovementComponent|AddInputVector (Variables|Default|GetMovementComponent) (Math|Vector|RotateVector ActionValue (Math|Rotator|MakeRotator 0.0 0.0 (.yaw (Transformation|GetActorRotation)))) false))

(event Input|EnhancedActionEvents|EnhancedInputActionIA_Rotate
  (params (ActionValue :type Vector%202D%20Structure) (ElapsedSeconds :type Float%20%28double-precision%29) (TriggeredSeconds :type Float%20%28double-precision%29) (InputAction :type Input%20Action%20Object%20Reference :default "/Game/DroneGame/Blueprints/Player/Input/IA_Rotate.IA_Rotate"))
  (Pawn|Input|AddControllerYawInput (.x ActionValue))
  (Pawn|Input|AddControllerPitchInput (.y ActionValue)))

(event Input|EnhancedActionEvents|EnhancedInputActionIA_Fire
  (params (ActionValue :type Boolean) (ElapsedSeconds :type Float%20%28double-precision%29) (TriggeredSeconds :type Float%20%28double-precision%29) (InputAction :type Input%20Action%20Object%20Reference :default "/Game/DroneGame/Blueprints/Player/Input/IA_Fire.IA_Fire"))
  (bind _weaponcomponent (Variables|Default|GetWeaponComponent))
  (:Started
    (Class|WeaponComponent|StartFire _weaponcomponent))
  (:Canceled
    (Class|WeaponComponent|StopFire _weaponcomponent :!label _label))
  (:Completed
    (goto _label)))

(fn ConstructionScript)